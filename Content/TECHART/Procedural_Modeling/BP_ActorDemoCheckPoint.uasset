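; Procedural modeling demo actor that scatters and removes sphere static mesh actors on demand.
; AddSpheres spawns about a hundred StaticMeshActors at random XY positions within a Boundary range at fixed height, assigns a sphere mesh and records each in ExistingSpheres.
; DeleteSpheres destroys every recorded actor but does not clear the array.
; BeginPlay, Tick and the construction script do nothing.
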(event Custom|Add%20Spheres
  (bind _boundary (Variables|Default|GetBoundary))
  (bind _boundary_2 (Variables|Default|GetBoundary))
  (for _index (range 0 100)
    (bind _returnvalue (Game|SpawnActorfromClass "/Script/Engine.StaticMeshActor" (Math|Transform|MakeTransform (Math|Vector|MakeVector (Math|Random|RandomFloatinRange (* _boundary_2 -1.0) _boundary_2) (Math|Random|RandomFloatinRange (* _boundary -1.0) _boundary) 5e+02)) "Undefined" "MultiplyWithRoot" 0 0))
    (Utilities|Array|Add (Variables|Default|GetExisting%20Spheres) _returnvalue)
    (Components|StaticMesh|SetStaticMesh (Variables|/Script/Engine.StaticMeshActor|GetStaticMeshComponent _returnvalue) "/Game/TECHART/Procedural_Modeling/Sphere_4B36049F.Sphere_4B36049F")))

(event Custom|Delete%20Spheres
  (for _array_element (Variables|Default|GetExisting%20Spheres)
    (Actor|DestroyActor _array_element)))

(event EventBeginPlay)

(event Collision|EventActorBeginOverlap
  (params (OtherActor :type Actor%20Object%20Reference)))

(event EventTick
  (params (DeltaSeconds :type Float%20%28single-precision%29)))

(fn ConstructionScript)