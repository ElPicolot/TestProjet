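; BP_ActorDemo is a procedural placement demo that scatters sphere meshes randomly within a boundary around the actor.
; The construction script adds up to CountBalls material-assigned mesh components, using a minimum-distance test against stored transforms, though Distance is never cleared between candidates.
; AddSpheres separately spawns tracked StaticMeshActors at fixed height, deriving both X and Y from the actor's X.
; DeleteSpheres destroys those, then destroys this actor if matching sphere actors are found.
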(event Custom|Add%20Spheres
  (bind _self self)
  (bind _boundary (Variables|Default|GetBoundary))
  (bind _boundary_2 (Variables|Default|GetBoundary))
  (bind _returnvalue (Transformation|GetActorLocation _self))
  (for _index (range 0 100)
    (bind _returnvalue_2 (Game|SpawnActorfromClass "/Script/Engine.StaticMeshActor" (Math|Transform|MakeTransform (Math|Vector|MakeVector (+ (.x _returnvalue) (Math|Random|RandomFloatinRange (* _boundary_2 -1.0) _boundary_2)) (+ (.x _returnvalue) (Math|Random|RandomFloatinRange (* _boundary -1.0) _boundary)) 5e+02)) "Undefined" "MultiplyWithRoot" 0 0))
    (Utilities|Array|Add (Variables|Default|GetExisting%20Spheres) _returnvalue_2)
    (Components|StaticMesh|SetStaticMesh (Variables|/Script/Engine.StaticMeshActor|GetStaticMeshComponent _returnvalue_2) "/Game/TECHART/Procedural_Modeling/_GENERATED/GAME3/Sphere_4B36049F.Sphere_4B36049F")))

(event Custom|Delete%20Spheres
  (Utilities|FlowControl|Sequence
    (:then_0
      (for _array_element (Variables|Default|GetExisting%20Spheres)
        (Actor|DestroyActor _array_element)))
    (:then_1
      (bind _outactors (Actor|GetAllActorsOfClass "/Script/Engine.StaticMeshActor"))
      (for _array_element_2 _outactors
        (if (== (Variables|/Script/Engine.StaticMeshComponent|GetStaticMesh (Variables|/Script/Engine.StaticMeshActor|GetStaticMeshComponent _array_element_2)) "/Game/TECHART/Procedural_Modeling/_GENERATED/GAME3/Sphere_4B36049F.Sphere_4B36049F")
          (Actor|DestroyActor))))))

(event EventBeginPlay)

(event Collision|EventActorBeginOverlap
  (params (OtherActor :type Actor%20Object%20Reference)))

(event EventTick
  (params (DeltaSeconds :type Float%20%28single-precision%29)))

(fn ConstructionScript
  (bind _boundary (Variables|Default|GetBoundary))
  (bind _boundary_2 (Variables|Default|GetBoundary))
  (Utilities|Array|Add (Variables|Default|GetTransform) (Transformation|GetActorTransform self))
  (for _index (range 0 (Variables|Default|GetCountBalls))
    (Variables|Default|SetTest%20Transform (Math|Transform|MakeTransform (Math|Vector|MakeVector (Math|Random|RandomFloatinRange (* _boundary -1.0) _boundary) (Math|Random|RandomFloatinRange (* _boundary_2 -1.0) _boundary_2) 0.0)))
    (for _array_element (Variables|Default|GetTransform)
      (Utilities|Array|Add (Variables|Default|GetDistance) (Math|Vector|Distance(Vector) (.Location (Math|Transform|BreakTransform _array_element)) (.Location (Math|Transform|BreakTransform (Variables|Default|GetTest%20Transform))))))
    (if (> (.MinValue (Math|Float|MinOfFloatArray (Variables|Default|GetDistance))) 1e+02)
      (bind _returnvalue (AddComponent|AddStaticMeshComponent false (Variables|Default|GetTest%20Transform)))
      (Components|StaticMesh|SetStaticMesh _returnvalue "/Game/TECHART/Procedural_Modeling/_GENERATED/GAME3/Sphere_4B36049F.Sphere_4B36049F")
      ;[1 1 1] Add Perso Mat Instance
      (Rendering|Material|SetMaterial _returnvalue 0 "/Game/TECHART/Tools/ToolsTest/RepriseP2/M_MannequinUE4_ChestLogo1.M_MannequinUE4_ChestLogo1")
      (Utilities|Array|Add (Variables|Default|GetTransform) (Variables|Default|GetTest%20Transform)))))